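; BP_Cannon is a cannon actor that automatically fires on a repeating cycle from BeginPlay.
; After a configurable delay, it spawns a scaled projectile at the Arrow component's location and rotation.
; It then plays CannonFireTimeline to animate the barrel mesh along its relative Y axis.
; The timeline's Cannon Fired output loops back to the delay, so firing repeats without using Tick.
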(event EventBeginPlay
  (Utilities|FlowControl|Delay (Variables|CannonProperties|GetProjectitlesDuration) :!label _label)
  (CallFunction|SpawnProjectile)
  (bind _cannonbarrellocation (Timeline|Cannon%20Fire%20Timeline PlayFromStart)
    (:Update
      (CallFunction|SetCannonAnimationLocation _cannonbarrellocation))
    (:CannonFired
      (goto _label))))

(event Collision|EventActorBeginOverlap
  (params (OtherActor :type Actor%20Object%20Reference)))

(event EventTick
  (params (DeltaSeconds :type Float%20%28single-precision%29)))

(fn ConstructionScript)

(fn SpawnProjectile
  (bind _arrow (Variables|Default|GetArrow))
  (bind _returnvalue (Transformation|GetWorldTransform _arrow))
  (Game|SpawnActorfromClass "/Game/NewFolder/Blueprints/Projectiles/BP_Projectiles.BP_Projectiles_C" (Math|Transform|MakeTransform (.location _returnvalue) (.rotation _returnvalue) (Math|Conversions|ToVector(Float) (Variables|CannonProperties|GetProjectile%20Scale))) "Undefined" 0 0))

(fn SetCannonAnimationLocation
  (params (CannonBarrelYLocation :type Float%20%28single-precision%29))
  (Transformation|SetRelativeLocation (Variables|Default|GetCanonn) (Math|Vector|MakeVector 0.0 CannonBarrelYLocation 0.0) false false))