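; BP_WinVolum is a level exit volume that completes the level when the player overlaps it after every crystal is gone.
; If any BPCrystal actors remain in the world, it moves the player pawn back to StartPlace instead.
; On completion, it finds the current level in the LevelsName array and opens the next entry, wrapping to the first after the final level.
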(event EventBeginPlay)

(event Collision|EventActorBeginOverlap
  (params (OtherActor :type Actor%20Object%20Reference))
  (Utilities|IsPlayer OtherActor
    (:IsPlayer
      (if (Pure|CheckAnyCrystal)
        (Impure|CompleteLevel)
        (else
          (Transformation|SetActorLocation (Game|Player|GetPlayerPawn 0) (Variables|Default|GetStartPlace) false false))))))

(event EventTick
  (params (DeltaSeconds :type Float%20%28single-precision%29)))

(fn ConstructionScript)

(fn CheckAnyCrystal
  (bind _outactors (Actor|GetAllActorsOfClass "/Game/NewFolder/Blueprints/Actor/Crystals/BPCrystal.BPCrystal_C"))
  (return (== (Utilities|Array|Length _outactors) 0)))

(fn CompleteLevel
  (if (Pure|IsFinalLevel)
    (Impure|OpenFirstLevel)
    (else
      (Impure|OpenNextLevel))))

(fn GetCurrentLevelIndex
  (bind _returnvalue (Game|GetCurrentLevelName true))
  (return (Utilities|Array|FindItem (Variables|Default|GetLevelsName) (Utilities|String|StringToName _returnvalue))))

(fn IsFinalLevel
  (return (== (Impure|GetCurrentLevelIndex) (Utilities|Array|LastIndex (Variables|Default|GetLevelsName)))))

(fn OpenFirstLevel
  (Game|OpenLevel(byName) (Pure|GetFirtsLevelName)))

(fn OpenNextLevel
  (Game|OpenLevel(byName) (Pure|GetNextLevelName)))

(fn GetNextLevelName
  (bind _levelsname (Variables|Default|GetLevelsName))
  (bind _returnvalue (Game|GetCurrentLevelName true))
  (return (Utilities|Array|Get(acopy) _levelsname (+ (Utilities|Array|FindItem _levelsname (Utilities|String|StringToName _returnvalue)) 1))))

(fn GetFirtsLevelName
  (return (Utilities|Array|Get(acopy) (Variables|Default|GetLevelsName))))