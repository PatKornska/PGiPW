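; BPPawn01 is a physics-driven rolling sphere pawn that restarts the level when it takes any damage.
; Forward/backward and left/right axis inputs share one torque node on the Sphere, scaled by StrMulti and applied as an acceleration change.
; The camera fades in on BeginPlay, while ResetLevel fades out, waits, then reopens the current level by name.
; Escape quits the game.
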(event Game|Damage|EventAnyDamage
  (params (Damage :type Float%20%28single-precision%29) (DamageType :type Damage%20Type%20Object%20Reference) (InstigatedBy :type Controller%20Object%20Reference) (DamageCauser :type Actor%20Object%20Reference))
  (Utilities|ResetLevel))

(event EventBeginPlay
  (CameraFades|StartCameraFade :self (Game|GetPlayerCameraManager 0) :FromAlpha 2.0 :Duration 2.0 :bHoldWhenFinished true))

(event Input|AxisEvents|InputAxisMoveForwardBackward
  (params (AxisValue :type Float%20%28single-precision%29))
  (bind _str_multi (Variables|Default|GetStr%20Multi))
  (Class|PrimitiveComponent|AddTorqueinRadians (Variables|Default|GetSphere) (Math|Vector|MakeVector (* (stale Input|AxisEvents|InputAxisMoveLeftRight AxisValue) _str_multi) (* AxisValue _str_multi) 0.0) "None" true))

(event Input|AxisEvents|InputAxisMoveLeftRight
  (params (AxisValue :type Float%20%28single-precision%29))
  (bind _str_multi (Variables|Default|GetStr%20Multi))
  (Class|PrimitiveComponent|AddTorqueinRadians (Variables|Default|GetSphere) (Math|Vector|MakeVector (* AxisValue _str_multi) (* (stale Input|AxisEvents|InputAxisMoveForwardBackward AxisValue) _str_multi) 0.0) "None" true))

(event Input|KeyboardEvents|Escape
  (params (Key :type Key%20Structure))
  (:Pressed
    (Game|QuitGame 0 "Quit")))

(fn ConstructionScript)